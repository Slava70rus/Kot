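; BP_Gun is a motion-controller gun that can be picked up and fires BP_Bullet projectiles.
; Pickup, called by BP_MotionController, attaches the gun to the given component, sets a fixed relative rotation and registers it as the player MotionControllerPawn's Gun.
; Shoot spawns a bullet at the Sphere component's location and rotation.
; Drop is empty, with its detach node left unconnected, so the gun stays attached.
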(event Custom|Shoot
  (bind _sphere (Variables|Default|GetSphere))
  (bind _returnvalue (Transformation|GetWorldTransform _sphere))
  (Game|SpawnActorfromClass "/Game/Items/BP_Bullet.BP_Bullet_C" (Math|Transform|MakeTransform (.location _returnvalue) (.rotation _returnvalue) "1,1,1") "Undefined" 0 0))

(event EventPickup
  (params (AttachTo :type Scene%20Component%20Object%20Reference))
  (Transformation|AttachComponentToComponent (VehicleSound|GetRootComponent) AttachTo "None" "KeepWorld" "KeepWorld" "KeepWorld" false)
  (Transformation|SetActorRelativeTransform (Math|Transform|MakeTransform "0, 0, 0" "0,-90.000000, 0" "1,1,1") false false)
  (bind _asmotion_controller_pawn (Utilities|Casting|CastToMotionControllerPawn (Game|Player|GetPlayerPawn 0)))
  (Variables|/Game/VirtualRealityBP/Blueprints/MotionControllerPawn.MotionControllerPawn_C|SetGun _asmotion_controller_pawn self))

(event EventDrop)

(fn ConstructionScript)