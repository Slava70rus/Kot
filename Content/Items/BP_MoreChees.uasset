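; BP_MoreChees is an item Blueprint that shows a Chees count on a text render and triggers a loss when that count runs out.
; The construction script writes the starting value to the text.
; RemoveChees decrements the count by one, refreshes the text and opens the Lose level when the count equals exactly zero.
; The event graph holds no active logic, so RemoveChees relies on an external caller.
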(event EventBeginPlay)

(event Collision|EventActorBeginOverlap
  (params (OtherActor :type Actor%20Object%20Reference)))

(event EventTick
  (params (DeltaSeconds :type Float%20%28single-precision%29)))

(fn ConstructionScript
  (Rendering|Components|TextRender|SetText (Variables|Default|GetTextRender) (Utilities|Text|ToText(Float) (Variables|Default|GetChees) "HalfToEven")))

(fn RemoveChees
  (bind _output_get (Variables|Default|SetChees (- (Variables|Default|GetChees) 1.0)))
  (Rendering|Components|TextRender|SetText (Variables|Default|GetTextRender) (Utilities|Text|ToText(Float) _output_get "HalfToEven"))
  (if (== _output_get 0.0)
    (Game|OpenLevel(byName) "Lose")))